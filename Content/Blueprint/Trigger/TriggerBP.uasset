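; TriggerBP is an interaction trigger that tells an overlapping actor when it is facing the trigger and exposes a set of montages through GetMontages.
; Its collision component stores a single overlapping actor, then clears it after sending an end-overlap message on exit.
; Each Tick compares that actor's yaw to the direction toward the trigger within a 50-degree tolerance, repeatedly sending begin or end overlap messages accordingly.
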(event `self.ReceiveTick`
  (params (DeltaSeconds :type "Float (single-precision)"))
  (bind _actor (`self.Actor`))
  (bind _actor_2 (`self.Actor`)
    (:`then`
      (bind _returnvalue (`self.GetTransform` _actor_2))
      (bind (_returnvalue_roll _returnvalue_pitch _returnvalue_yaw) (`KismetMathLibrary.BreakRotator` (`KismetMathLibrary.Conv_VectorToRotator` (- (`self.K2_GetActorLocation`) (.location _returnvalue)))))
      (if (== (`KismetMathLibrary.MakeRotator` 0.0 0.0 (.yaw (.rotation _returnvalue))) (`KismetMathLibrary.MakeRotator` 0.0 0.0 _returnvalue_yaw) :`ErrorTolerance` 50.0)
        (message `/Game/Blueprint/Interface/TriggerInterface.BeginOverlap` _actor self)
        (else
          (message `/Game/Blueprint/Interface/TriggerInterface.EndOverlap` _actor self))))
    (:`else`)))

(event `self.CollisionComponent.OnComponentBeginOverlap`
  (params (OverlappedComponent :type "PrimitiveComponent Object Reference") (OtherActor :type "Actor Object Reference") (OtherComp :type "PrimitiveComponent Object Reference") (OtherBodyIndex :type Integer) (bFromSweep :type Boolean) (SweepResult :type "HitResult Structure (by ref)"))
  (set `self.Actor` OtherActor))

(event `self.CollisionComponent.OnComponentEndOverlap`
  (params (OverlappedComponent :type "PrimitiveComponent Object Reference") (OtherActor :type "Actor Object Reference") (OtherComp :type "PrimitiveComponent Object Reference") (OtherBodyIndex :type Integer))
  (message `/Game/Blueprint/Interface/TriggerInterface.EndOverlap` OtherActor self)
  (set `self.Actor` null))

(fn `GetMontages`
  (returns (Montages :type "AnimMontage Object Reference"))
  (return (`self.Montages`)))

(fn `UserConstructionScript`)