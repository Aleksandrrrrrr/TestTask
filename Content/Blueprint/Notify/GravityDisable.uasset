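; GravityDisable is an animation notify state that suspends gravity on a character for a span of an animation.
; On begin it casts the mesh owner to Character and switches its movement mode to Flying.
; On end it sets the mode to Falling so gravity resumes, without restoring whatever mode was active before.
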(fn `Received_NotifyBegin`
  (params (MeshComp :type "SkeletalMeshComponent Object Reference") (Animation :type "AnimSequenceBase Object Reference") (TotalDuration :type "Float (double-precision)"))
  (returns (ReturnValue :type Boolean))
  (`CharacterMovementComponent.SetMovementMode` (`Character.CharacterMovement` (cast `Character` (`ActorComponent.GetOwner` MeshComp) :!pure true)) "MOVE_Flying" 0)
  (return false))

(fn `Received_NotifyEnd`
  (params (MeshComp :type "SkeletalMeshComponent Object Reference") (Animation :type "AnimSequenceBase Object Reference"))
  (returns (ReturnValue :type Boolean))
  (`CharacterMovementComponent.SetMovementMode` (`Character.CharacterMovement` (cast `Character` (`ActorComponent.GetOwner` MeshComp) :!pure true)) "MOVE_Falling" 0)
  (return false))